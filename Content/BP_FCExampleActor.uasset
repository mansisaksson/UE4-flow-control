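; BP_FCExampleActor is an example actor that demonstrates asynchronous lerp nodes for float, vector and rotator values.
; On BeginPlay it chains the three timed lerps through their "then" outputs, printing each interpolated value on that node's Tick output.
; A Condition function reports whether game time has passed a fixed threshold, but nothing in these graphs calls it.
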(event EventBeginPlay
  (bind _value (|LerpFloat 0.0 1e+01 5.0)
    (:then
      (bind _value_2 (Math|Vector|Lerp(Vector) "0, 0, 0" "100.000000,100.000000,100.000000" 5.0)
        (:then
          (bind _value_3 (Math|Rotator|Lerp(Rotator) "0, 0, 0" "0,90.000000, 0" 5.0)
            (:Tick
              (Development|PrintString (Utilities|String|ToString(Rotator) _value_3)))))
        (:Tick
          (Development|PrintString (Utilities|String|ToString(Vector) _value_2)))))
    (:Tick
      (Development|PrintString (Utilities|String|ToString(Float) _value)))))

(event Collision|EventActorBeginOverlap
  (params (OtherActor :type Actor%20Object%20Reference)))

(event EventTick
  (params (DeltaSeconds :type Float%20%28single-precision%29)))

(fn ConstructionScript)

(fn Condition
  (return (> (Utilities|Time|GetGameTimeinSeconds) 5.0)))